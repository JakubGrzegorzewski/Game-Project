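; Burning damage-over-time style status effect Blueprint that shows a fire visual on the affected character.
; On apply, it calls the parent logic, then attaches a Niagara burning system to the target's root component and stores it.
; On remove, it calls the parent logic and destroys that component if valid.
; The target's StatsComponent validity checks lead to no action, so any over-time behaviour is not in this graph.
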(event EventOnApply
  (bind _returnvalue (Class|StatusEffect|GetTargetCharacter))
  (|CallParentFunction)
  (bind _returnvalue_2 (Niagara|SpawnSystemAttached "/Game/Blueprints/VFX/NS_Free_Magic_Burning.NS_Free_Magic_Burning" (Variables|/Script/Engine.Actor|GetRootComponent (Class|StatusEffect|GetTargetCharacter)) "None" "0, 0, 0" "0, 0, 0" "SnapToTarget" true))
  (Variables|Default|SetNiagara _returnvalue_2)
  (Utilities|IsValid _returnvalue
    (:Is%20Valid
      (Variables|/Script/GameProject.BaseCharacter|GetStatsComponent _returnvalue
        (:then)
        (:else)))))

(event EventOnRemove
  (|CallParentFunction)
  (bind _niagara (Variables|Default|GetNiagara)
    (:then
      (Components|DestroyComponent _niagara))
    (:else)))