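; Sprint status effect that temporarily raises the target character's walk speed while it is active.
; On apply, it caches the movement component's current max speed and sets MaxWalkSpeed to that plus the spec's Magnitude.
; It also attaches a magic-circle Niagara system to the character's root and stores the reference.
; On removal, it restores the cached speed but does not explicitly stop the Niagara system.
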(event EventOnRemove
  (bind _returnvalue (Class|StatusEffect|GetTargetCharacter))
  (|CallParentFunction)
  (Utilities|IsValid _returnvalue
    (:Is%20Valid
      (Variables|/Script/Engine.CharacterMovementComponent|SetMaxWalkSpeed (Variables|/Script/Engine.Character|GetCharacterMovement _returnvalue) (Variables|Default|GetMaxSpeed)))))

(event EventOnApply
  (bind _returnvalue (Class|StatusEffect|GetTargetCharacter))
  (bind _charactermovement (Variables|/Script/Engine.Character|GetCharacterMovement _returnvalue))
  (bind _returnvalue_2 (Class|MovementComponent|GetMaxSpeed _charactermovement))
  (|CallParentFunction)
  (Utilities|IsValid _returnvalue
    (:Is%20Valid
      (Variables|Default|SetMaxSpeed _returnvalue_2)
      (Variables|/Script/Engine.CharacterMovementComponent|SetMaxWalkSpeed _charactermovement (+ _returnvalue_2 (Utilities|Struct|BreakStatusEffectSpec (Class|StatusEffect|GetSpec))))
      (bind _returnvalue_3 (Niagara|SpawnSystemAttached "/Game/Blueprints/VFX/NS_Free_Magic_Circle2.NS_Free_Magic_Circle2" (Variables|/Script/Engine.Actor|GetRootComponent (Class|StatusEffect|GetTargetCharacter)) "None" "0, 0, 0" "0, 0, 0" "KeepRelativeOffset" true))
      (Variables|Default|SetNiagara _returnvalue_3))))